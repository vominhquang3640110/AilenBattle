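; BP_ChangeModeItem is a spinning pickup that switches the overlapping BP_Character to a random mode.
; On BeginPlay the authority calls a multicast-named event that rolls the mode and spin direction inside its body, while Tick applies the spin.
; The first character overlapping the box receives the mode through ChangeMode (called twice) and ChangeStatus, then the item destroys itself.
; The pickup sound component is destroyed immediately after spawning.
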(event OnComponentBeginOverlap(Box)
  (params (OverlappedComponent :type Primitive%20Component%20Object%20Reference) (OtherActor :type Actor%20Object%20Reference) (OtherComp :type Primitive%20Component%20Object%20Reference) (OtherBodyIndex :type Integer) (bFromSweep :type Boolean) (SweepResult :type Hit%20Result%20Structure%20%28by%20ref%29))
  ;[1 1 1] Get This Item
  (if (not (Variables|Default|GetWasUsed))
    (bind _asbp_character (Utilities|Casting|CastToBP_Character OtherActor))
    (Variables|Default|SetWasUsed true)
    (bind _returnvalue (Audio|SpawnSoundatLocation "/Game/AilenBattle/Sound/SC_PickupItem.SC_PickupItem" (Transformation|GetActorLocation) "0, 0, 0" 1.0 1.0 0.0 0 0))
    (Components|DestroyComponent _returnvalue)
    (bind _output_get (Variables|/Game/AilenBattle/Blueprints/InGame/BP_Character.BP_Character_C|SetModeNumber _asbp_character (Variables|Default|GetModeNumber)))
    (Default|ChangeMode _asbp_character _output_get)
    (Default|ChangeStatus _asbp_character _output_get)
    (Default|ChangeMode _asbp_character _output_get)
    (Actor|DestroyActor)))

(event Custom|SetModeNumber_Multicast
  (Variables|Default|SetModeNumber (Math|Random|RandomIntegerinRange 1 3))
  (Variables|Default|SetRotation (Math|Random|RandomBool)))

(event EventBeginPlay
  (if (not (Variables|Default|GetWasSetModeNumber))
    (Variables|Default|SetWasSetModeNumber true)
    (Networking|SwitchHasAuthority
      (:Authority
        (CallFunction|SetModeNumberMulticast)))))

(event EventTick
  (params (DeltaSeconds :type Float%20%28single-precision%29))
  (if (Variables|Default|GetRotation)
    (Transformation|AddActorLocalRotation "0.000000,1.000000,0.000000" false false)
    (else
      (Transformation|AddActorLocalRotation "0.000000,-1.000000,0.000000" false false))))

(fn ConstructionScript)