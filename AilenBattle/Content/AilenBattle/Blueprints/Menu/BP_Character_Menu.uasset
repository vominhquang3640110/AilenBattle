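; Menu character that switches its appearance between its original look and three modes: defense/speed-up, attack/speed-up and one-kill/speed-down.
; On BeginPlay it caches materials and skeletal meshes from the main Mesh and three extra skeletal mesh components, which serve as per-mode templates.
; ChangeModeChar advances a wrapping mode index, and ChangeMode applies that mode's mesh and dynamic material instances to the main Mesh, recording it as current.
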(event Custom|ChangeModeChar
  (bind _result (Math|Integer|IncrementInt (Variables|Default|GetModeNumber))
    (:%20%20
      (if (< _result 4)
        _
        (else
          (Variables|Default|SetModeNumber 0)))
      (CallFunction|ChangeMode (Variables|Default|GetModeNumber)))))

(event EventBeginPlay
  (CallFunction|SetModeSkeletalMaterial))

(fn ConstructionScript)

(fn ChangeMode
  (params (ModeNumber :type Integer))
  (bind _oldmodematerial (Variables|Default|GetOldModeMaterial))
  (bind _defspeed_up_modematerial (Variables|Default|GetDefSpeed_Up_ModeMaterial))
  (bind _atkspeed_up_modematerial (Variables|Default|GetAtkSpeed_Up_ModeMaterial))
  (bind _onekillspeed_down_modematerial (Variables|Default|GetOnekillSpeed_Down_ModeMaterial))
  (bind (_materials _skeletalmesh) (Utilities|Struct|BreakCharacterSM _oldmodematerial))
  (bind (_materials_2 _skeletalmesh_2) (Utilities|Struct|BreakCharacterSM _defspeed_up_modematerial))
  (bind (_materials_3 _skeletalmesh_3) (Utilities|Struct|BreakCharacterSM _atkspeed_up_modematerial))
  (bind (_materials_4 _skeletalmesh_4) (Utilities|Struct|BreakCharacterSM _onekillspeed_down_modematerial))
  (bind _returnvalue (Utilities|Select :Index ModeNumber :Option%200 _materials :Option%201 _materials_2 :Option%202 _materials_3 :Option%203 _materials_4))
  (bind _returnvalue_2 (Utilities|Select :Index ModeNumber :Option%200 _skeletalmesh :Option%201 _skeletalmesh_2 :Option%202 _skeletalmesh_3 :Option%203 _skeletalmesh_4))
  (for (_array_element _array_index) _returnvalue
    (Rendering|Material|CreateDynamicMaterialInstance (Variables|Character|GetMesh) _array_index _array_element "None" :!class /Script/Engine.PrimitiveComponent)
    (Components|SkeletalMesh|SetSkeletalMeshAsset (Variables|Character|GetMesh) _returnvalue_2)
    (Variables|Default|SetNowModeMaterial (Utilities|Struct|MakeCharacterSM _returnvalue _returnvalue_2))))

(fn SetModeSkeletalMaterial
  (bind _mesh (Variables|Character|GetMesh))
  (bind _skeletalmesh2 (Variables|Default|GetSkeletalMesh2))
  (bind _mesh_2 (Variables|Character|GetMesh))
  (bind _skeletalmesh (Variables|Default|GetSkeletalMesh))
  (bind _skeletalmesh1 (Variables|Default|GetSkeletalMesh1))
  (Variables|Default|SetNowModeMaterial (Utilities|Struct|MakeCharacterSM (Rendering|Material|GetMaterials _mesh_2) (Components|SkeletalMesh|GetSkeletalMeshAsset _mesh_2)))
  (Variables|Default|SetOldModeMaterial (Utilities|Struct|MakeCharacterSM (Rendering|Material|GetMaterials _mesh) (Components|SkeletalMesh|GetSkeletalMeshAsset _mesh)))
  (Variables|Default|SetDefSpeed_Up_ModeMaterial (Utilities|Struct|MakeCharacterSM (Rendering|Material|GetMaterials _skeletalmesh) (Components|SkeletalMesh|GetSkeletalMeshAsset _skeletalmesh)))
  (Variables|Default|SetAtkSpeed_Up_ModeMaterial (Utilities|Struct|MakeCharacterSM (Rendering|Material|GetMaterials _skeletalmesh1) (Components|SkeletalMesh|GetSkeletalMeshAsset _skeletalmesh1)))
  (Variables|Default|SetOnekillSpeed_Down_ModeMaterial (Utilities|Struct|MakeCharacterSM (Rendering|Material|GetMaterials _skeletalmesh2) (Components|SkeletalMesh|GetSkeletalMeshAsset _skeletalmesh2)))
  (return))