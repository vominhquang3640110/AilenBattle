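; BP_SpawnChangeModeItem is a spawner that scatters BP_ChangeModeItem pickups inside its bounds once the match starts.
; Tick polls player 0's BP_Character for IsStartGame, latches IsStartPawn, then waits ten seconds before the first wave.
; SpawnItem loops five times, picking a random point and yaw for SpawnOnSever to spawn at.
; SpawnOnSever then delays by SpawnTime and calls SpawnItem again, repeating waves indefinitely.
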(event Custom|SpawnItem
  (bind (_origin _boxextent) (Collision|GetActorBounds false false))
  (bind _isstartpawn (Variables|Default|GetIsStartPawn))
  (for _array_element (Utilities|Array|MakeArray _isstartpawn _isstartpawn _isstartpawn _isstartpawn _isstartpawn)
    (Variables|Default|SetSpawnTransform (Math|Transform|MakeTransform (Math|Random|RandomPointinBoundingBox _origin _boxextent) (Math|Rotator|MakeRotator 0.0 0.0 (Math|Random|RandomFloatinRange 0.0 3.6e+02))))
    (CallFunction|SpawnonSever)))

(event Custom|SpawnOnSever
  (Game|SpawnActorfromClass "/Game/AilenBattle/Blueprints/InGame/BP_ChangeModeItem.BP_ChangeModeItem_C" (Variables|Default|GetSpawnTransform) "Undefined" "MultiplyWithRoot" 0 0)
  (Utilities|FlowControl|Delay (Variables|Default|GetSpawnTime))
  (CallFunction|SpawnItem))

(event EventBeginPlay)

(event Collision|EventActorBeginOverlap
  (params (OtherActor :type Actor%20Object%20Reference)))

(event EventTick
  (params (DeltaSeconds :type Float%20%28single-precision%29))
  (if (not (Variables|Default|GetIsStartPawn))
    (bind _asbp_character (Utilities|Casting|CastToBP_Character (Game|GetPlayerCharacter 0)))
    (if (Variables|/Game/AilenBattle/Blueprints/InGame/BP_Character.BP_Character_C|GetisStartGame _asbp_character)
      (Variables|Default|SetIsStartPawn true)
      (Utilities|FlowControl|Delay 1e+01)
      (CallFunction|SpawnItem))))

(fn ConstructionScript)