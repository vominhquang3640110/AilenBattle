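; BP_ProjectileInGame is an arrow-like projectile that plays a fire sound on spawn and rotates to follow its velocity.
; On its first character hit it spawns an actor, notifies the local player's HUD if that player was hit, then OnSever subtracts GiveDame from clamped HP and destroys it.
; On other hits it freezes in place without collision, plays an impact sound unless it struck an explosion box, and is destroyed after a short delay.
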(event Custom|OnSever
  ;[1 1 1] Hit Event
  ;;[0.03813 0.03499 0.1844] Comment
  (Variables|/Game/AilenBattle/Blueprints/InGame/BP_Character.BP_Character_C|SetHP (stale Collision|EventHit _asbp_character) (Math|Float|Clamp(Float) (- (Variables|/Game/AilenBattle/Blueprints/InGame/BP_Character.BP_Character_C|GetHP (stale Collision|EventHit _asbp_character)) (Variables|Default|GetGiveDame))))
  (Actor|DestroyActor))

(event Collision|EventHit
  (params (MyComp :type Primitive%20Component%20Object%20Reference) (Other :type Actor%20Object%20Reference) (OtherComp :type Primitive%20Component%20Object%20Reference) (bSelfMoved :type Boolean) (HitLocation :type Vector :default "0, 0, 0") (HitNormal :type Vector :default "0, 0, 0") (NormalImpulse :type Vector :default "0, 0, 0") (Hit :type Hit%20Result%20Structure%20%28by%20ref%29))
  (bind _box (Variables|Default|GetBox))
  ;[1 1 1] Hit Event
  ;;[0.03813 0.03499 0.1844] Comment
  (bind _asbp_character (Utilities|Casting|CastToBP_Character Other)
    (:then
      (if (not (Variables|Default|GetIsGiveDame))
        (Variables|Default|SetIsGiveDame true)
        (Game|SpawnActorfromClass "/Game/AilenBattle/Blueprints/InGame/BP_HitEffect.BP_HitEffect_C" (Transformation|GetActorTransform) "Undefined" "MultiplyWithRoot" 0 0)
        (if (== _asbp_character (Game|GetPlayerCharacter 0))
          (Default|GetDame (Variables|/Game/AilenBattle/Blueprints/InGame/BP_Character.BP_Character_C|GetHUBRef _asbp_character)))
        (CallFunction|OnSever)))
    (:CastFailed
      ;;[0.6219 0.554 0.1049] Actor
      (Utilities|Casting|CastToBP_ExplosionBox Other
        (:then
          _)
        (:CastFailed
          (bind _returnvalue (Audio|SpawnSoundatLocation "/Game/AilenBattle/Sound/SC_ArrowHit.SC_ArrowHit" (Transformation|GetActorLocation) "0, 0, 0" 1.0 1.0 0.0 0 0))
          (Components|DestroyComponent _returnvalue)))
      (Variables|Default|SetNowRotation (Transformation|GetActorTransform))
      (Variables|/Script/Engine.ProjectileMovementComponent|SetbSimulationEnabled (Variables|Default|GetProjectileMovement) false)
      (Physics|SetSimulatePhysics _box false)
      (Collision|SetCollisionEnabled _box "NoCollision")
      (Transformation|SetActorTransform (Variables|Default|GetNowRotation))
      (Utilities|FlowControl|Delay 1.0)
      (Actor|DestroyActor))))

(event EventBeginPlay
  (bind _returnvalue (Audio|SpawnSoundatLocation "/Game/AilenBattle/Sound/SC_Fire.SC_Fire" (Transformation|GetActorLocation) "0, 0, 0" 1.0 1.0 0.0 0 0))
  (Components|DestroyComponent _returnvalue))

(event EventTick
  (params (DeltaSeconds :type Float%20%28single-precision%29))
  ;[1 1 1] Rotator Update
  (if (Variables|/Script/Engine.ProjectileMovementComponent|GetbSimulationEnabled (Variables|Default|GetProjectileMovement))
    (Transformation|SetActorRotation (Math|Rotator|MakeRotfromX (Transformation|GetVelocity)))))

(fn ConstructionScript)

(fn OnRepGiveDame)