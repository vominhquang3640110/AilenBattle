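; BP_ExplosionBox is an explosive box actor that detonates when hit by a BP_ProjectileInGame.
; The hit destroys the projectile, enables the initially collisionless Sphere as a blast area and spawns BP_ExplosionEffect.
; Once activated, Tick subtracts GiveDame from the normalized HP of every overlapping BP_Character, then destroys the box, even if none overlap.
; On destruction it spawns an explosion sound, then immediately destroys that audio component.
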(event EventTick
  (params (DeltaSeconds :type Float%20%28single-precision%29))
  (bind _overlappingactors (Collision|GetOverlappingActors "/Game/AilenBattle/Blueprints/InGame/BP_Character.BP_Character_C" :!class /Script/Engine.Actor))
  (if (Variables|Default|GetwasActived)
    (if (> (Utilities|Array|Length _overlappingactors) 0)
      (for (_array_element _array_index) _overlappingactors
        (bind _asbp_character (Utilities|Casting|CastToBP_Character _array_element))
        (Variables|/Game/AilenBattle/Blueprints/InGame/BP_Character.BP_Character_C|SetHP _asbp_character (Math|Float|Clamp(Float) (- (Variables|/Game/AilenBattle/Blueprints/InGame/BP_Character.BP_Character_C|GetHP _asbp_character) (Variables|Default|GetGiveDame))))
        (if (== _array_index (- (Utilities|Array|Length _overlappingactors) 1))
          (Actor|DestroyActor)))
      (else
        (Actor|DestroyActor)))))

(event EventDestroyed
  (bind _returnvalue (Audio|SpawnSoundatLocation "/Game/AilenBattle/Sound/SC_Explosion.SC_Explosion" (Transformation|GetActorLocation) "0, 0, 0" 1.0 1.0 0.0 0 0))
  (Components|DestroyComponent _returnvalue))

(event Collision|EventHit
  (params (MyComp :type Primitive%20Component%20Object%20Reference) (Other :type Actor%20Object%20Reference) (OtherComp :type Primitive%20Component%20Object%20Reference) (bSelfMoved :type Boolean) (HitLocation :type Vector :default "0, 0, 0") (HitNormal :type Vector :default "0, 0, 0") (NormalImpulse :type Vector :default "0, 0, 0") (Hit :type Hit%20Result%20Structure%20%28by%20ref%29))
  (bind _asbp_projectile_in_game (Utilities|Casting|CastToBP_ProjectileInGame Other))
  (Variables|Default|SetwasActived true)
  (Actor|DestroyActor _asbp_projectile_in_game)
  (Collision|SetCollisionEnabled (Variables|Default|GetSphere) "QueryAndPhysics")
  (Game|SpawnActorfromClass "/Game/AilenBattle/Blueprints/InGame/BP_ExplosionEffect.BP_ExplosionEffect_C" (Transformation|GetActorTransform) "Undefined" "MultiplyWithRoot" 0 0))

(event EventBeginPlay
  (Collision|SetCollisionEnabled (Variables|Default|GetSphere) "NoCollision"))

(fn ConstructionScript)